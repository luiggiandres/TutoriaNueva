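; BP_Pistola is a pistol the player character can equip and drop.
; Its Collision overlap events enable and disable the actor's input for player 0, without checking which actor overlaps.
; EQUIPAR snaps it to the character mesh's RHSocket, and DEJAR detaches it, keeping its world transform.
; Both actions cast to BP_Militar to switch its ModoAccionActual action mode.
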(event `self.Collision.OnComponentBeginOverlap`
  (params (OverlappedComponent :type "PrimitiveComponent Object Reference") (OtherActor :type "Actor Object Reference") (OtherComp :type "PrimitiveComponent Object Reference") (OtherBodyIndex :type Integer) (bFromSweep :type Boolean) (SweepResult :type "HitResult Structure (by ref)"))
  (`self.EnableInput` (`GameplayStatics.GetPlayerController` 0)))

(event `self.Collision.OnComponentEndOverlap`
  (params (OverlappedComponent :type "PrimitiveComponent Object Reference") (OtherActor :type "Actor Object Reference") (OtherComp :type "PrimitiveComponent Object Reference") (OtherBodyIndex :type Integer))
  (`self.DisableInput` (`GameplayStatics.GetPlayerController` 0)))

(event `InputAction|EQUIPAR`
  (params (Key :type "Key Structure"))
  (:`Pressed`
    (`self.Equipar`)))

(event `InputAction|DEJAR`
  (params (Key :type "Key Structure"))
  (:`Pressed`
    (`self.Dejar`)))

(fn `Dejar`
  (bind _asbp_militar (cast `/Game/ThirdPerson/Blueprints/BP_Militar` (`GameplayStatics.GetPlayerCharacter` 0)))
  (`self.K2_DetachFromActor` "KeepWorld" "KeepWorld" "KeepWorld")
  (set `/Game/ThirdPerson/Blueprints/BP_Militar.ModoAccionActual` "NewEnumerator0" _asbp_militar))

(fn `Equipar`
  (bind _returnvalue (`GameplayStatics.GetPlayerCharacter` 0))
  (`self.K2_AttachToComponent` (`Character.Mesh` _returnvalue) "RHSocket" "SnapToTarget" "SnapToTarget" "SnapToTarget")
  (bind _asbp_militar (cast `/Game/ThirdPerson/Blueprints/BP_Militar` _returnvalue))
  (set `/Game/ThirdPerson/Blueprints/BP_Militar.ModoAccionActual` "NewEnumerator1" _asbp_militar))

(fn `UserConstructionScript`)