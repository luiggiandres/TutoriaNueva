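; BP_Enemigo is an AI enemy character that flags a pursuit when it sees a pawn.
; PawnSensing sets the Blackboard key "Siguiendo" to true on any sighting, with no class filter, and nothing here clears it.
; Tick switches walk speed between walking and running from the Corriendo flag, which this graph never sets.
; A leftover, unconnected call to damage BP_Militar never runs.
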(event `self.ReceiveTick`
  (params (DeltaSeconds :type "Float (single-precision)"))
  (bind _charactermovement (`self.CharacterMovement`))
  ;[1 1 1] Regula la velocidad c
  (if (`self.Corriendo`)
    (set `CharacterMovementComponent.MaxWalkSpeed` 370.0 _charactermovement)
    (else
      (set `CharacterMovementComponent.MaxWalkSpeed` 150.0 _charactermovement))))

(event `self.PawnSensing.OnSeePawn`
  (params (Pawn :type "Pawn Object Reference"))
  (`BlackboardComponent.SetValueAsBool` (`AIBlueprintHelperLibrary.GetBlackboard` self) "Siguiendo" true))

(fn `UserConstructionScript`)